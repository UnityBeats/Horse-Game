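; Checkpoint trigger actor that saves the player's position when they walk into its Box.
; On overlap by a FirstPersonCharacter, it records that character's location into LastLocation of a CheckpointSave object.
; It loads the existing "CheckpointSlot" save or creates a new one, then writes it back to that slot.
; The stored point is the character's location at overlap, not the checkpoint's own; loading it for respawn is not handled here.
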(event OnComponentBeginOverlap(Box)
  (params (OverlappedComponent :type Primitive%20Component%20Object%20Reference) (OtherActor :type Actor%20Object%20Reference) (OtherComp :type Primitive%20Component%20Object%20Reference) (OtherBodyIndex :type Integer) (bFromSweep :type Boolean) (SweepResult :type Hit%20Result%20Structure%20%28by%20ref%29))
  (bind _asfirst_person_character (Utilities|Casting|CastToFirstPersonCharacter OtherActor))
  (Variables|Default|SetLocation (Transformation|GetActorLocation _asfirst_person_character))
  (bind _returnvalue (SaveGame|DoesSaveGameExist "CheckpointSlot"))
  (if _returnvalue
    (bind _returnvalue_2 (SaveGame|LoadGamefromSlot "CheckpointSlot"))
    (bind _output_get (Variables|Default|SetSaveSubClass _returnvalue_2))
    (bind _ascheckpoint_save (Utilities|Casting|CastToCheckpointSave _output_get))
    (Variables|/Game/CheckpointSave.CheckpointSave_C|SetLastLocation _ascheckpoint_save (Variables|Default|GetLocation))
    (SaveGame|SaveGametoSlot (Variables|Default|GetSaveSubClass) "CheckpointSlot")
    (else
      (bind _returnvalue_3 (SaveGame|CreateSaveGameObject "/Game/CheckpointSave.CheckpointSave_C"))
      (bind _output_get_2 (Variables|Default|SetSaveSubClass _returnvalue_3))
      (bind _ascheckpoint_save_2 (Utilities|Casting|CastToCheckpointSave _output_get_2))
      (Variables|/Game/CheckpointSave.CheckpointSave_C|SetLastLocation _ascheckpoint_save_2 (Variables|Default|GetLocation))
      (SaveGame|SaveGametoSlot (Variables|Default|GetSaveSubClass) "CheckpointSlot"))))

(event EventBeginPlay)

(event Collision|EventActorBeginOverlap
  (params (OtherActor :type Actor%20Object%20Reference)))

(event EventTick
  (params (DeltaSeconds :type Float%20%28single-precision%29)))

(fn ConstructionScript)